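; Behavior tree task that performs the zombie's melee attack on the player character.
; It reads the zombie from the SelfActor blackboard key, plays an attack sound and montage, and lowers the zombie's roaming audio until the montage ends.
; A montage notify applies random damage if the TargetActor player overlaps the zombie's damage collision.
; The task succeeds on montage completion and fails on interruption.
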(event EventReceiveExecute
  (params (OwnerActor :type Actor%20Object%20Reference))
  ;[1 1 1] 为了创建蒙太奇与动作转换为Character
  (bind _asbp_zombie_1 (Utilities|Casting|CastToBP_Zombie1 (Class|BTFunctionLibrary|GetBlackboardValueasObject (Utilities|Struct|MakeBlackboardKeySelector 0 "SelfActor" "/Script/AIModule.BlackboardKeyType_Object" 255 false))))
  (Audio|Components|Audio|SetVolumeMultiplier (Variables|/Game/FPS_game/Characters/BP_Zombie1.BP_Zombie1_C|GetRadioRoaming _asbp_zombie_1) 0.15 :!class /Script/Engine.AudioComponent)
  (Audio|PlaySound2D "/Game/FPS_game/Characters/Male_Zombie/zombie_attack_sound.zombie_attack_sound" 1.0 1.0 0.0 0 0)
  (Animation|Montage|PlayMontage (Variables|/Script/Engine.Character|GetMesh _asbp_zombie_1) "/Game/FPS_game/Characters/Male_Zombie/AM_Zombie1.AM_Zombie1"
    (:OnCompleted
      (AI|BehaviorTree|FinishExecute true)
      (Audio|Components|Audio|SetVolumeMultiplier (Variables|/Game/FPS_game/Characters/BP_Zombie1.BP_Zombie1_C|GetRadioRoaming _asbp_zombie_1) 1.0 :!class /Script/Engine.AudioComponent :!label _label))
    (:OnInterrupted
      (AI|BehaviorTree|FinishExecute false)
      (goto _label))
    (:OnNotifyBegin
      (bind _asbp_fpscharacter_1 (Utilities|Casting|CastToBP_FPSCharacter1 (Class|BTFunctionLibrary|GetBlackboardValueasObject (Utilities|Struct|MakeBlackboardKeySelector 0 "TargetActor" "/Script/AIModule.BlackboardKeyType_Object" 255 false))))
      (if (Collision|IsOverlappingActor (Variables|/Game/FPS_game/Characters/BP_Zombie1.BP_Zombie1_C|GetDamageCollusion _asbp_zombie_1) _asbp_fpscharacter_1 :!class /Script/Engine.PrimitiveComponent)
        (Game|Damage|ApplyDamage _asbp_fpscharacter_1 (Math|Random|RandomFloatinRange 15.0 25.0) 0 0)))))