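; FPS game mode for a timed round where the player must kill all BP_Zombie1 enemies to win.
; BeginPlay creates the HUD, counts zombies and disables player input.
; Tick runs a warmup countdown, then the round timer, which turns red near zero, driven by a session state.
; ZombieDied, PlayerDied and timeout set win or loss states, update HUD announcements and disable input on the player pawn.
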(event EventBeginPlay
  (bind _gamemodehudref (Variables|Default|GetGameModeHUDRef))
  (Utilities|FlowControl|Sequence
    (:then_0
      (CallFunction|AddGameModeHUD))
    (:then_1
      ;[1 1 1] 更新敌人数量
      (bind _outactors (Actor|GetAllActorsOfClass "/Game/FPS_game/Characters/BP_Zombie1.BP_Zombie1_C"))
      (Rendering|Components|TextRender|SetText (Variables|/Game/FPS_game/Blueprints/UI/W_GameModeHUD1.W_GameModeHUD1_C|GetZombiesCount_Text (Variables|Default|GetGameModeHUDRef)) (Utilities|Text|ToText(Integer) (Utilities|Array|Length _outactors)))
      (Variables|Default|SetZombieCount (Utilities|Array|Length _outactors)))
    (:then_2
      (bind _asbp_fpscharacter_1 (Utilities|Casting|CastToBP_FPSCharacter1 (Game|Player|GetPlayerPawn 0)))
      (Input|DisableInput _asbp_fpscharacter_1 (Game|GetPlayerController 0))
      (Variables|/Game/FPS_game/Characters/BP_FPSCharacter1.BP_FPSCharacter1_C|SetPrimaryActionPressed _asbp_fpscharacter_1 false)
      (Rendering|Components|TextRender|SetText (Variables|/Game/FPS_game/Blueprints/UI/W_GameModeHUD1.W_GameModeHUD1_C|GetTimeRemaining_Text _gamemodehudref) (CallFunction|FormatText))
      (Rendering|Components|TextRender|SetText (Variables|/Game/FPS_game/Blueprints/UI/W_GameModeHUD1.W_GameModeHUD1_C|GetAnnouncement_Text _gamemodehudref) "规定时间内击杀所有敌人"))))

(event EventTick
  (params (DeltaSeconds :type Float%20%28single-precision%29))
  (switch Utilities|FlowControl|Switch|SwitchonE_SessionState1 (Variables|Default|GetSessionState)
    (:NewEnumerator0
      (CallFunction|WarmupTimer))
    (:NewEnumerator1
      (CallFunction|UpdateCountdownTimer DeltaSeconds))))

(fn ConstructionScript)

(fn ZombieDied
  ;[1 1 1] 击败敌人计数减一
  (bind _result (Math|Integer|DecrementInt (Variables|Default|GetZombieCount))
    (:%20%20
      (Rendering|Components|TextRender|SetText (Variables|/Game/FPS_game/Blueprints/UI/W_GameModeHUD1.W_GameModeHUD1_C|GetZombiesCount_Text (Variables|Default|GetGameModeHUDRef)) (Utilities|Text|ToText(Integer) _result))
      (if (<= (Variables|Default|GetZombieCount) 0)
        (CallFunction|PlayerWon)))))

(fn WarmupTimer
  (bind _returnvalue (Utilities|Time|GetGameTimeinSeconds))
  (bind _gamemodehudref (Variables|Default|GetGameModeHUDRef))
  (bind _warmuptime (Variables|Default|GetWarmupTime))
  (bind _returnvalue_2 (- _warmuptime _returnvalue))
  (bind _countdown_text (Variables|/Game/FPS_game/Blueprints/UI/W_GameModeHUD1.W_GameModeHUD1_C|GetCountdown_text _gamemodehudref))
  (bind _returnvalue_3 (Class|KismetMathLibrary|FCeil64 _returnvalue_2))
  (Rendering|Components|TextRender|SetText _countdown_text (Utilities|Text|ToText(String) _returnvalue_3))
  ;[1 1 1] 倒计时后可以开始游戏
  (if (<= _returnvalue_3 0)
    (Rendering|Components|TextRender|SetText _countdown_text "")
    (CallFunction|StartGame)))

(fn StartGame
  (Rendering|Components|TextRender|SetText (Variables|/Game/FPS_game/Blueprints/UI/W_GameModeHUD1.W_GameModeHUD1_C|GetAnnouncement_Text (Variables|Default|GetGameModeHUDRef)) "")
  (bind _asbp_fpscharacter_1 (Utilities|Casting|CastToBP_FPSCharacter1 (Game|Player|GetPlayerPawn 0)))
  (Input|EnableInput _asbp_fpscharacter_1 (Game|GetPlayerController 0))
  (Variables|Default|SetSessionState "NewEnumerator1"))

(fn UpdateCountdownTimer
  (params (DeltaTime :type Float%20%28double-precision%29))
  (bind _gamemodehudref (Variables|Default|GetGameModeHUDRef))
  (bind _timeremaining_text (Variables|/Game/FPS_game/Blueprints/UI/W_GameModeHUD1.W_GameModeHUD1_C|GetTimeRemaining_Text _gamemodehudref))
  (bind _output_get (Variables|Default|SetCountdownTime (- (Variables|Default|GetCountdownTime) DeltaTime)))
  (Rendering|Components|TextRender|SetText _timeremaining_text (CallFunction|FormatText))
  (if (<= _output_get 11.0)
    (Appearance|SetColorandOpacity _timeremaining_text (Utilities|Struct|MakeSlateColor "(R=1.000000,G=0.000000,B=0.000000,A=1.000000)" "UseColor_Specified") :!class /Script/UMG.TextBlock)
    (if (<= _output_get 0.0)
      (CallFunction|OutOfTime))))

(fn OutOfTime
  (bind _returnvalue (Game|Player|GetPlayerPawn 0))
  (Rendering|Components|TextRender|SetText (Variables|/Game/FPS_game/Blueprints/UI/W_GameModeHUD1.W_GameModeHUD1_C|GetTimeRemaining_Text (Variables|Default|GetGameModeHUDRef)) "00:00")
  (Variables|Default|SetSessionState "NewEnumerator2")
  (bind _asbp_fpscharacter_1 (Utilities|Casting|CastToBP_FPSCharacter1 _returnvalue))
  (Input|DisableInput _returnvalue 0)
  (Variables|/Game/FPS_game/Characters/Main_Arms/ABP_AK_47_arms1.ABP_AK_47_arms1_C|SetIsAiming (Variables|/Game/FPS_game/Characters/BP_FPSCharacter1.BP_FPSCharacter1_C|GetABPAK47Arms1 _asbp_fpscharacter_1) false)
  (Transformation|SetRelativeLocationAndRotation (Variables|/Game/FPS_game/Characters/BP_FPSCharacter1.BP_FPSCharacter1_C|GetArmMesh _asbp_fpscharacter_1) (Variables|/Game/FPS_game/Characters/BP_FPSCharacter1.BP_FPSCharacter1_C|GetNotAimingPosition _asbp_fpscharacter_1) (Variables|/Game/FPS_game/Characters/BP_FPSCharacter1.BP_FPSCharacter1_C|GetNotAimingRotation _asbp_fpscharacter_1) false false)
  (Rendering|Components|TextRender|SetText (Variables|/Game/FPS_game/Blueprints/UI/W_GameModeHUD1.W_GameModeHUD1_C|GetAnnouncement_Text (Variables|Default|GetGameModeHUDRef)) "超出时间限制"))

(fn FormatText
  (bind _countdowntime (Variables|Default|GetCountdownTime))
  (bind _returnvalue (/ _countdowntime 6e+01))
  (bind _returnvalue_2 (Math|Float|Floor _returnvalue))
  (return (Utilities|Text|FormatText "{Minutes}:{Seconds}" (Utilities|Text|ToText(Integer) _returnvalue_2 false true 2 2) (Utilities|Text|ToText(Integer) (Math|Float|Floor (- (Variables|Default|GetCountdownTime) (* _returnvalue_2 60))) false true 2 2))))

(fn AddGameModeHUD
  ;[1 1 1] 添加控件
  (bind _returnvalue (UserInterface|CreateWidget "/Game/FPS_game/Blueprints/UI/W_GameModeHUD1.W_GameModeHUD1_C"))
  (bind _output_get (Variables|Default|SetGameModeHUDRef _returnvalue))
  (UserInterface|Viewport|AddtoViewport _output_get 0))

(fn PlayerWon
  (bind _returnvalue (Game|Player|GetPlayerPawn 0))
  (Variables|Default|SetSessionState "NewEnumerator4")
  (bind _asbp_fpscharacter_1 (Utilities|Casting|CastToBP_FPSCharacter1 _returnvalue))
  (if (> (Variables|/Game/FPS_game/Characters/BP_FPSCharacter1.BP_FPSCharacter1_C|GetHealth _asbp_fpscharacter_1) 0.0)
    (Input|DisableInput _returnvalue (Game|GetPlayerController 0))
    (Variables|/Game/FPS_game/Characters/BP_FPSCharacter1.BP_FPSCharacter1_C|SetPrimaryActionPressed _asbp_fpscharacter_1 false)
    (Rendering|Components|TextRender|SetText (Variables|/Game/FPS_game/Blueprints/UI/W_GameModeHUD1.W_GameModeHUD1_C|GetAnnouncement_Text (Variables|Default|GetGameModeHUDRef)) "获得胜利")))

(fn PlayerDied
  (Variables|Default|SetSessionState "NewEnumerator3")
  (bind _asbp_fpscharacter_1 (Utilities|Casting|CastToBP_FPSCharacter1 (Game|Player|GetPlayerPawn 0)))
  (Input|DisableInput _asbp_fpscharacter_1 (Game|GetPlayerController 0))
  (Variables|/Game/FPS_game/Characters/BP_FPSCharacter1.BP_FPSCharacter1_C|SetPrimaryActionPressed _asbp_fpscharacter_1 false)
  (Rendering|Components|TextRender|SetText (Variables|/Game/FPS_game/Blueprints/UI/W_GameModeHUD1.W_GameModeHUD1_C|GetAnnouncement_Text (Variables|Default|GetGameModeHUDRef)) "游戏失败"))