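; Game mode for a timed FPS zombie round in which the player must kill every BP_Zombie before the countdown expires.
; BeginPlay creates the HUD, counts zombies and disables player input until a warmup ends.
; Tick switches on SessionState to run the warmup or countdown, whose display turns red near zero.
; ZombieDied decrements the count toward a win, while timeout and PlayerDied end the round with input disabled and an announcement.
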(event EventBeginPlay
  (bind _returnvalue (Game|Player|GetPlayerPawn 0))
  (bind _gamemodehudref (Variables|Default|GetGameModeHUDRef))
  (Utilities|FlowControl|Sequence
    (:then_0
      (CallFunction|AddGameModeHUD))
    (:then_1
      (bind _outactors (Actor|GetAllActorsOfClass "/Game/FPS_game/Characters/BP_Zombie.BP_Zombie_C"))
      (Rendering|Components|TextRender|SetText (Variables|/Game/FPS_game/Blueprints/UI/W_GameModeHUD.W_GameModeHUD_C|GetZombiesCount_Text (Variables|Default|GetGameModeHUDRef)) (Utilities|Text|ToText(Integer) (Utilities|Array|Length _outactors)))
      (Variables|Default|SetZombieCount (Utilities|Array|Length _outactors)))
    (:then_2
      (bind _asbp_fpscharacter (Utilities|Casting|CastToBP_FPSCharacter _returnvalue))
      (Input|DisableInput _returnvalue 0)
      (Variables|/Game/FPS_game/Characters/BP_FPSCharacter.BP_FPSCharacter_C|SetPrimaryActionPressed _asbp_fpscharacter false)
      (Rendering|Components|TextRender|SetText (Variables|/Game/FPS_game/Blueprints/UI/W_GameModeHUD.W_GameModeHUD_C|GetTimeRemaining_Text _gamemodehudref) (CallFunction|FormatText))
      (Rendering|Components|TextRender|SetText (Variables|/Game/FPS_game/Blueprints/UI/W_GameModeHUD.W_GameModeHUD_C|GetAnnouncement_Text _gamemodehudref) "Kill all the zombies!"))))

(event EventTick
  (params (DeltaSeconds :type Float%20%28single-precision%29))
  (switch Utilities|FlowControl|Switch|SwitchonE_SessionState (Variables|Default|GetSessionState)
    (:NewEnumerator0
      (CallFunction|WarmupTimer))
    (:NewEnumerator1
      (CallFunction|UpdateCountdownTimer DeltaSeconds))))

(fn ConstructionScript)

(fn ZombieDied
  (bind _result (Math|Integer|DecrementInt (Variables|Default|GetZombieCount))
    (:%20%20
      (Rendering|Components|TextRender|SetText (Variables|/Game/FPS_game/Blueprints/UI/W_GameModeHUD.W_GameModeHUD_C|GetZombiesCount_Text (Variables|Default|GetGameModeHUDRef)) (Utilities|Text|ToText(Integer) _result))
      (if (<= (Variables|Default|GetZombieCount) 0)
        (CallFunction|PlayerWon)))))

(fn WarmupTimer
  (bind _returnvalue (Utilities|Time|GetGameTimeinSeconds))
  (bind _warmuptime (Variables|Default|GetWarmupTime))
  (bind _returnvalue_2 (- _warmuptime _returnvalue))
  (bind _returnvalue_3 (Class|KismetMathLibrary|FCeil64 _returnvalue_2))
  (Rendering|Components|TextRender|SetText (Variables|/Game/FPS_game/Blueprints/UI/W_GameModeHUD.W_GameModeHUD_C|GetCountdown_text (Variables|Default|GetGameModeHUDRef)) (Utilities|Text|ToText(String) _returnvalue_3))
  (if (<= _returnvalue_3 0)
    (Rendering|Components|TextRender|SetText (Variables|/Game/FPS_game/Blueprints/UI/W_GameModeHUD.W_GameModeHUD_C|GetCountdown_text (Variables|Default|GetGameModeHUDRef)) "")
    (CallFunction|StartGame)))

(fn StartGame
  (bind _asbp_fpscharacter (Utilities|Casting|CastToBP_FPSCharacter (Game|Player|GetPlayerPawn 0)))
  (Input|EnableInput _asbp_fpscharacter (Game|GetPlayerController 0))
  (Variables|Default|SetSessionState "NewEnumerator1")
  (Rendering|Components|TextRender|SetText (Variables|/Game/FPS_game/Blueprints/UI/W_GameModeHUD.W_GameModeHUD_C|GetAnnouncement_Text (Variables|Default|GetGameModeHUDRef)) ""))

(fn UpdateCountdownTimer
  (params (DeltaTime :type Float%20%28double-precision%29))
  (bind _output_get (Variables|Default|SetCountdownTime (- (Variables|Default|GetCountdownTime) DeltaTime)))
  (Rendering|Components|TextRender|SetText (Variables|/Game/FPS_game/Blueprints/UI/W_GameModeHUD.W_GameModeHUD_C|GetTimeRemaining_Text (Variables|Default|GetGameModeHUDRef)) (CallFunction|FormatText))
  (if (<= _output_get 1e+01)
    (Appearance|SetColorandOpacity (Variables|/Game/FPS_game/Blueprints/UI/W_GameModeHUD.W_GameModeHUD_C|GetTimeRemaining_Text (Variables|Default|GetGameModeHUDRef)) (Utilities|Struct|MakeSlateColor "(R=1.000000,G=0.000000,B=0.000000,A=1.000000)" "UseColor_Specified") :!class /Script/UMG.TextBlock)
    (if (<= _output_get 0.0)
      (CallFunction|OutOfTime))))

(fn OutOfTime
  (bind _returnvalue (Game|Player|GetPlayerPawn 0))
  (Rendering|Components|TextRender|SetText (Variables|/Game/FPS_game/Blueprints/UI/W_GameModeHUD.W_GameModeHUD_C|GetTimeRemaining_Text (Variables|Default|GetGameModeHUDRef)) "00:00")
  (Variables|Default|SetSessionState "NewEnumerator2")
  (bind _asbp_fpscharacter (Utilities|Casting|CastToBP_FPSCharacter _returnvalue))
  (Input|DisableInput _returnvalue 0)
  (Variables|/Game/FPS_game/Characters/BP_FPSCharacter.BP_FPSCharacter_C|SetPrimaryActionPressed _asbp_fpscharacter false)
  (Rendering|Components|TextRender|SetText (Variables|/Game/FPS_game/Blueprints/UI/W_GameModeHUD.W_GameModeHUD_C|GetAnnouncement_Text (Variables|Default|GetGameModeHUDRef)) "Out of Time!"))

(fn FormatText
  (bind _countdowntime (Variables|Default|GetCountdownTime))
  (bind _returnvalue (/ _countdowntime 6e+01))
  (bind _returnvalue_2 (Math|Float|Floor _returnvalue))
  (return (Utilities|Text|FormatText "{Minutes}:{Seconds}" (Utilities|Text|ToText(Integer) _returnvalue_2 false true 2 2) (Utilities|Text|ToText(Float) (- (Variables|Default|GetCountdownTime) (* _returnvalue_2 60)) "HalfToEven" false true 2 2 0 0))))

(fn AddGameModeHUD
  (bind _returnvalue (Game|ConstructObjectfromClass "/Game/FPS_game/Blueprints/UI/W_GameModeHUD.W_GameModeHUD_C"))
  (Variables|Default|SetGameModeHUDRef _returnvalue)
  (UserInterface|Viewport|AddtoViewport _returnvalue 0))

(fn PlayerWon
  (bind _returnvalue (Game|Player|GetPlayerPawn 0))
  (Variables|Default|SetSessionState "NewEnumerator4")
  (bind _asbp_fpscharacter (Utilities|Casting|CastToBP_FPSCharacter _returnvalue))
  (if (not (<= (Variables|/Game/FPS_game/Characters/BP_FPSCharacter.BP_FPSCharacter_C|GetHealth _asbp_fpscharacter) 0.0))
    (Input|DisableInput _returnvalue 0)
    (Variables|/Game/FPS_game/Characters/BP_FPSCharacter.BP_FPSCharacter_C|SetPrimaryActionPressed _asbp_fpscharacter false)
    (Rendering|Components|TextRender|SetText (Variables|/Game/FPS_game/Blueprints/UI/W_GameModeHUD.W_GameModeHUD_C|GetAnnouncement_Text (Variables|Default|GetGameModeHUDRef)) "You Won!")))

(fn PlayerDied
  (bind _gamemodehudref (Variables|Default|GetGameModeHUDRef))
  (Variables|Default|SetSessionState "NewEnumerator3")
  (bind _asbp_fpscharacter (Utilities|Casting|CastToBP_FPSCharacter (Game|Player|GetPlayerPawn 0)))
  (Input|DisableInput _asbp_fpscharacter 0)
  (Variables|/Game/FPS_game/Characters/BP_FPSCharacter.BP_FPSCharacter_C|SetPrimaryActionPressed _asbp_fpscharacter false)
  (Rendering|Components|TextRender|SetText (Variables|/Game/FPS_game/Blueprints/UI/W_GameModeHUD.W_GameModeHUD_C|GetAnnouncement_Text _gamemodehudref) "You Died!")
  (Rendering|Components|TextRender|SetText (Variables|/Game/FPS_game/Blueprints/UI/W_GameModeHUD.W_GameModeHUD_C|GetTimeRemaining_Text _gamemodehudref) "00:00"))