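; BP_Zombie1 is an enemy zombie with randomized health that chases the player and explodes after dying.
; Player overlap with PlayerDetect or incoming damage writes the target to the Blackboard's TargetActor for the AI.
; At zero health, the ZombieDies macro stops AI and movement, plays death effects and notifies FPS_game_mode1.
; After a delay, Explode damages the detected player if inside ExplodeCollusion, then destroys the zombie.
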(event OnComponentBeginOverlap(PlayerDetect)
  (params (OverlappedComponent :type Primitive%20Component%20Object%20Reference) (OtherActor :type Actor%20Object%20Reference) (OtherComp :type Primitive%20Component%20Object%20Reference) (OtherBodyIndex :type Integer) (bFromSweep :type Boolean) (SweepResult :type Hit%20Result%20Structure%20%28by%20ref%29))
  ;[1 1 1] 创建追踪玩家所需要的TargetActor
  (bind _asbp_fpscharacter_1 (Utilities|Casting|CastToBP_FPSCharacter1 OtherActor))
  (bind _output_get (Variables|Default|SetAsBPFPSCharacter1 _asbp_fpscharacter_1))
  (Utilities|FlowControl|DoOnce false
    (:Completed
      (Development|PrintString "开始追踪玩家")
      (AI|Components|Blackboard|SetValueasObject (AI|GetBlackboard (AI|GetAIController self)) (Utilities|Name|MakeLiteralName "TargetActor") _output_get))))

(event EventBeginPlay
  (Variables|Default|SetHealth (Math|Random|RandomFloatinRange 8e+01 1.5e+02)))

(event Game|Damage|EventAnyDamage
  (params (Damage :type Float%20%28single-precision%29) (DamageType :type Damage%20Type%20Object%20Reference) (InstigatedBy :type Controller%20Object%20Reference) (DamageCauser :type Actor%20Object%20Reference))
  ;[1 1 1] 玩家攻击Zombie时追踪玩家
  (AI|Components|Blackboard|SetValueasObject (AI|GetBlackboard 0) (Utilities|Name|MakeLiteralName "TargetActor") DamageCauser)
  (if (> (Variables|Default|GetHealth) 0.0)
    (bind _output_get (Variables|Default|SetHealth (- (Variables|Default|GetHealth) Damage)))
    (if (<= _output_get 0.0)
      (Utilities|FlowControl|DoOnce false
        (:Completed
          (Utilities|ZombieDies))))))

(event EventTick
  (params (DeltaSeconds :type Float%20%28single-precision%29)))

(fn ConstructionScript)

(fn Explode
  (bind _returnvalue (Transformation|GetActorLocation))
  (bind _asbpfpscharacter1 (Variables|Default|GetAsBPFPSCharacter1))
  (Audio|SpawnSoundatLocation "/Game/StarterContent/Audio/Explosion_Cue.Explosion_Cue" _returnvalue "0, 0, 0" 1.0 1.0 0.0 0 0)
  (Effects|SpawnEmitteratLocation "/Game/StarterContent/Particles/P_Explosion.P_Explosion" _returnvalue "0, 0, 0" "1.500000,1.500000,1.500000")
  ;[1 1 1] 死亡爆炸对玩家造成伤害
  (if (Collision|IsOverlappingActor (Variables|Default|GetExplodeCollusion) _asbpfpscharacter1 :!class /Script/Engine.PrimitiveComponent)
    (Game|Damage|ApplyDamage _asbpfpscharacter1 3e+01 0 0)
    (Actor|DestroyActor)
    (else
      (Actor|DestroyActor))))